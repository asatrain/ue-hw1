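; BP_ConeR is an actor that rocks back and forth around its roll axis.
; Tick accumulates time and uses the parity of its rounded value to flip direction every second, starting with a half-second swing.
; Each frame it adds HalfAngle, scaled by direction and delta time, to the current roll, so HalfAngle acts as degrees per second while pitch and yaw are preserved.
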(event `self.ReceiveTick`
  (params (DeltaSeconds :type "Float (single-precision)"))
  (bind (_returnvalue_roll _returnvalue_pitch _returnvalue_yaw) (`KismetMathLibrary.BreakRotator` (`self.K2_GetActorRotation`)))
  (bind _output_get (set `self.time` (+ DeltaSeconds (`self.time`))))
  (if (!= (mod (`KismetMathLibrary.Round` _output_get) 2) 0)
    (set `self.rotationDirection` 1)
    (else
      (set `self.rotationDirection` -1)))
  (`self.K2_SetActorRotation` (`KismetMathLibrary.MakeRotator` (+ (* (* (`self.rotationDirection`) (`self.halfAngle`)) (`GameplayStatics.GetWorldDeltaSeconds`)) _returnvalue_roll) _returnvalue_pitch _returnvalue_yaw)))

(fn `UserConstructionScript`)