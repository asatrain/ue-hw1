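; BP_CubeR is an actor that moves by itself, alternating between turning in place and travelling forward.
; Tick accumulates elapsed time and uses the parity of the whole-second count to switch modes every second.
; Odd seconds add yaw at RotationAngle per second, while even seconds move the actor along its forward vector at Speed, without sweep.
; Both motions scale by world delta seconds.
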(event `self.ReceiveTick`
  (params (DeltaSeconds :type "Float (single-precision)"))
  (bind (_returnvalue_roll _returnvalue_pitch _returnvalue_yaw) (`KismetMathLibrary.BreakRotator` (`self.K2_GetActorRotation`)))
  (bind _output_get (set `self.time` (+ DeltaSeconds (`self.time`))))
  (if (!= (mod (`KismetMathLibrary.FFloor` _output_get) 2) 0)
    (`self.K2_SetActorRotation` (`KismetMathLibrary.MakeRotator` _returnvalue_roll _returnvalue_pitch (+ _returnvalue_yaw (* (`self.rotationAngle`) (`GameplayStatics.GetWorldDeltaSeconds`)))))
    (else
      (`self.K2_SetActorLocation` (+ (* (* (`self.GetActorForwardVector`) (`self.speed`)) (`GameplayStatics.GetWorldDeltaSeconds`)) (`self.K2_GetActorLocation`))))))

(fn `UserConstructionScript`)